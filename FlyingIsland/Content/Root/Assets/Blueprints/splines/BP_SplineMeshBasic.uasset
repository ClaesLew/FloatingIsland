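; Spline-driven fence builder that assembles poles and fence sections along an editable spline in the construction script.
; An instanced static mesh places a Pole at every spline point, optionally following the spline's rotation.
; Spline mesh components bend the Fence mesh between neighboring points with configurable forward axis and collision.
; An optional closed loop adds a last-to-first segment, which does not receive those axis and collision settings.
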(event EventBeginPlay)

(event Collision|EventActorBeginOverlap
  (params (OtherActor :type Actor%20Object%20Reference)))

(event EventTick
  (params (DeltaSeconds :type Float%20%28single-precision%29)))

(fn ConstructionScript
  (bind _spline (Variables|Default|GetSpline))
  (bind _spline_2 (Variables|Default|GetSpline))
  (bind _spline_3 (Variables|Default|GetSpline))
  (bind (_location _tangent) (Spline|GetLocationandTangentatSplinePoint _spline 0 "Local"))
  (bind _returnvalue (Spline|GetNumberOfSplinePoints _spline_3))
  (bind _returnvalue_2 (- _returnvalue 1))
  (bind (_location_2 _tangent_2) (Spline|GetLocationandTangentatSplinePoint _spline_2 _returnvalue_2 "Local"))
  (Utilities|FlowControl|Sequence
    (:then_0
      (Components|StaticMesh|SetStaticMesh (Variables|Default|GetInstancedStaticMesh) (Variables|Default|GetPole)))
    (:then_1
      (for _index (range 0 (- (Spline|GetNumberOfSplinePoints (Variables|Default|GetSpline)) 1))
        (if (Variables|Default|GetIsRotating)
          (Components|InstancedStaticMesh|AddInstance (Variables|Default|GetInstancedStaticMesh) (Spline|GetTransformatSplinePoint (Variables|Default|GetSpline) _index "Local" true))
          (else
            (Components|InstancedStaticMesh|AddInstance (Variables|Default|GetInstancedStaticMesh) (Math|Transform|MakeTransform (.Location (Math|Transform|BreakTransform (Spline|GetTransformatSplinePoint (Variables|Default|GetSpline) _index "Local" true))) "0, 0, 0" (.Scale (Math|Transform|BreakTransform (Spline|GetTransformatSplinePoint (Variables|Default|GetSpline) _index "Local" true)))))))))
    (:then_2
      (for _index_2 (range 0 (- (Spline|GetNumberOfSplinePoints (Variables|Default|GetSpline)) 2))
        (bind _returnvalue_3 (AddComponent|AddSplineMeshComponent false))
        (Components|StaticMesh|SetStaticMesh _returnvalue_3 (Variables|Default|GetFence))
        (SplineMesh|SetForwardAxis _returnvalue_3 (Variables|Default|GetSmForwardAxis) true)
        (Collision|SetCollisionEnabled _returnvalue_3 (Variables|Default|GetCollisionType))
        (SplineMesh|SetStartandEnd _returnvalue_3 (.Location (Spline|GetLocationandTangentatSplinePoint (Variables|Default|GetSpline) _index_2 "Local")) (.Tangent (Spline|GetLocationandTangentatSplinePoint (Variables|Default|GetSpline) _index_2 "Local")) (.Location (Spline|GetLocationandTangentatSplinePoint (Variables|Default|GetSpline) (+ _index_2 1) "Local")) (.Tangent (Spline|GetLocationandTangentatSplinePoint (Variables|Default|GetSpline) (+ _index_2 1) "Local")) true :!class /Script/Engine.SplineMeshComponent))
      (if (Variables|Default|GetbIsClosedLoop)
        (Spline|SetClosedLoop _spline_3 true true)
        (bind _returnvalue_4 (AddComponent|AddSplineMeshComponent false))
        (Components|StaticMesh|SetStaticMesh _returnvalue_4 (Variables|Default|GetFence))
        (SplineMesh|SetStartandEnd _returnvalue_4 _location_2 _tangent_2 _location _tangent true :!class /Script/Engine.SplineMeshComponent)
        (else
          (Spline|SetClosedLoop _spline_3 false true))))))