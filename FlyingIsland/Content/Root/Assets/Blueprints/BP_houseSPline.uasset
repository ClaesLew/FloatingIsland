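; Spline-driven actor that lays a static mesh along an editable spline, apparently for house-related pieces.
; The construction script adds one spline mesh component per segment, with configurable mesh, forward axis and collision, attached to the Scene component.
; Tangents come from each point's forward vector times its scale and the straight-line segment length, instead of the spline's own tangents.
; It has no runtime logic.
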(event EventBeginPlay)

(event Collision|EventActorBeginOverlap
  (params (OtherActor :type Actor%20Object%20Reference)))

(event EventTick
  (params (DeltaSeconds :type Float%20%28single-precision%29)))

(fn ConstructionScript
  (bind _spline (Variables|Default|GetSpline))
  (for _index (range 0 (- (Spline|GetNumberOfSplinePoints (Variables|Default|GetSpline)) 2))
    (bind _returnvalue (AddComponent|AddSplineMeshComponent false))
    (Components|StaticMesh|SetStaticMesh _returnvalue (Variables|Default|GetStaticMesh))
    (SplineMesh|SetForwardAxis _returnvalue (Variables|Default|GetSMC_ForwardAxis) true)
    (Collision|SetCollisionEnabled _returnvalue (Variables|Default|GetCollisionType))
    (Transformation|AttachComponentToComponent _returnvalue (Variables|Default|GetScene) "None" "KeepRelative" "KeepRelative" "KeepRelative" true)
    (SplineMesh|SetStartandEnd _returnvalue (.Location (Math|Transform|BreakTransform (Spline|GetTransformatSplinePoint _spline _index "Local" true))) (* (* (Math|Vector|GetForwardVector (.Rotation (Math|Transform|BreakTransform (Spline|GetTransformatSplinePoint _spline _index "Local" true)))) (.Scale (Math|Transform|BreakTransform (Spline|GetTransformatSplinePoint _spline _index "Local" true)))) (Math|Vector|VectorLength (- (.Location (Math|Transform|BreakTransform (Spline|GetTransformatSplinePoint _spline _index "Local" true))) (.Location (Math|Transform|BreakTransform (Spline|GetTransformatSplinePoint _spline (+ _index 1) "Local" true)))))) (.Location (Math|Transform|BreakTransform (Spline|GetTransformatSplinePoint _spline (+ _index 1) "Local" true))) (* (* (Math|Vector|GetForwardVector (.Rotation (Math|Transform|BreakTransform (Spline|GetTransformatSplinePoint _spline (+ _index 1) "Local" true)))) (.Scale (Math|Transform|BreakTransform (Spline|GetTransformatSplinePoint _spline (+ _index 1) "Local" true)))) (Math|Vector|VectorLength (- (.Location (Math|Transform|BreakTransform (Spline|GetTransformatSplinePoint _spline _index "Local" true))) (.Location (Math|Transform|BreakTransform (Spline|GetTransformatSplinePoint _spline (+ _index 1) "Local" true)))))) true :!class /Script/Engine.SplineMeshComponent)))