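; Master spline actor Blueprint that builds meshes along an editable spline in the Construction Script.
; Instanced static meshes place separate start and end meshes at the first and last spline points.
; Each segment gets a spline mesh component using first, middle or last mesh, with configurable forward axis and collision.
; Segment tangents are derived from point rotation and scale, multiplied by the straight-line distance between neighboring points.
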(event EventBeginPlay)

(event Collision|EventActorBeginOverlap
  (params (OtherActor :type Actor%20Object%20Reference)))

(event EventTick
  (params (DeltaSeconds :type Float%20%28single-precision%29)))

(fn ConstructionScript
  (bind _spline (Variables|Default|GetSpline))
  (bind _spline_2 (Variables|Default|GetSpline))
  (bind _spline_3 (Variables|Default|GetSpline))
  (bind _returnvalue (Spline|GetNumberOfSplinePoints _spline))
  (bind _returnvalue_2 (Spline|GetNumberOfSplinePoints _spline_2))
  (bind _returnvalue_3 (- _returnvalue 1))
  (bind _returnvalue_4 (- _returnvalue_2 2))
  (Utilities|FlowControl|Sequence
    (:then_0
      ;[1 1 1] Point Meshes
      (for _index (range 0 _returnvalue_3)
        (if (== _index 0)
          (Components|StaticMesh|SetStaticMesh (Variables|Default|GetInstancedStaticMesh) (Variables|Default|GetStartPointMesh))
          (Components|InstancedStaticMesh|AddInstance (Variables|Default|GetInstancedStaticMesh) (Math|Transform|MakeTransform (.Location (Math|Transform|BreakTransform (Spline|GetTransformatSplinePoint (Variables|Default|GetSpline) _index "Local" false))) "0, 0, 0" (.Scale (Math|Transform|BreakTransform (Spline|GetTransformatSplinePoint (Variables|Default|GetSpline) _index "Local" false)))))
          (Development|PrintString "Hello")
          (elif (== _index _returnvalue_3)
            (Components|StaticMesh|SetStaticMesh (Variables|Default|GetInstancedStaticMesh2) (Variables|Default|GetEndPointMesh))
            (Components|InstancedStaticMesh|AddInstance (Variables|Default|GetInstancedStaticMesh2) (Math|Transform|MakeTransform (.Location (Math|Transform|BreakTransform (Spline|GetTransformatSplinePoint (Variables|Default|GetSpline) _index "Local" false))) "0, 0, 0" (.Scale (Math|Transform|BreakTransform (Spline|GetTransformatSplinePoint (Variables|Default|GetSpline) _index "Local" false)))))
            (Development|PrintString "goodbye")))))
    (:then_1
      (for _index_2 (range 0 _returnvalue_4)
        (bind _returnvalue_5 (AddComponent|AddSplineMeshComponent false))
        ;[1 1 1] Tangent Meshes
        (Components|StaticMesh|SetStaticMesh _returnvalue_5 (Variables|Default|GetMidTangentMesh))
        (if (== _index_2 0)
          (Components|StaticMesh|SetStaticMesh _returnvalue_5 (Variables|Default|GetFirstTangentMesh))
          (elif (== _index_2 _returnvalue_4)
            (Components|StaticMesh|SetStaticMesh _returnvalue_5 (Variables|Default|GetLastTangentMesh))))
        (SplineMesh|SetForwardAxis _returnvalue_5 (Variables|Default|GetSMC_ForwardAxis) true)
        (Collision|SetCollisionEnabled _returnvalue_5 (Variables|Default|GetCollisionType))
        (Transformation|AttachComponentToComponent _returnvalue_5 (Variables|Default|GetScene) "None" "KeepRelative" "KeepRelative" "KeepRelative" true)
        (SplineMesh|SetStartandEnd _returnvalue_5 (.Location (Math|Transform|BreakTransform (Spline|GetTransformatSplinePoint _spline_3 _index_2 "Local" true))) (* (* (Math|Vector|GetForwardVector (.Rotation (Math|Transform|BreakTransform (Spline|GetTransformatSplinePoint _spline_3 _index_2 "Local" true)))) (.Scale (Math|Transform|BreakTransform (Spline|GetTransformatSplinePoint _spline_3 _index_2 "Local" true)))) (Math|Vector|VectorLength (- (.Location (Math|Transform|BreakTransform (Spline|GetTransformatSplinePoint _spline_3 _index_2 "Local" true))) (.Location (Math|Transform|BreakTransform (Spline|GetTransformatSplinePoint _spline_3 (+ _index_2 1) "Local" true)))))) (.Location (Math|Transform|BreakTransform (Spline|GetTransformatSplinePoint _spline_3 (+ _index_2 1) "Local" true))) (* (* (Math|Vector|GetForwardVector (.Rotation (Math|Transform|BreakTransform (Spline|GetTransformatSplinePoint _spline_3 (+ _index_2 1) "Local" true)))) (.Scale (Math|Transform|BreakTransform (Spline|GetTransformatSplinePoint _spline_3 (+ _index_2 1) "Local" true)))) (Math|Vector|VectorLength (- (.Location (Math|Transform|BreakTransform (Spline|GetTransformatSplinePoint _spline_3 _index_2 "Local" true))) (.Location (Math|Transform|BreakTransform (Spline|GetTransformatSplinePoint _spline_3 (+ _index_2 1) "Local" true)))))) true :!class /Script/Engine.SplineMeshComponent)))))